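; Spline-placed prop and lighting actor that builds a row of random meshes with spotlights along its spline.
; The construction script adds a randomly picked MeshArray spline mesh at each point, lowered and yawed by offsets, without setting start/end tangents.
; Every even point also gets an offset spotlight with shared color, cone angles and IES brightness scale.
; Helpers for spawning standalone StaticMeshActors exist but never run, as BeginPlay is empty.
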(event `self.ReceiveBeginPlay`)

(fn `Spawn`
  (bind _mesh_array (`self.Mesh_Array`))
  (for _index (range (`SplineComponent.GetNumberOfSplinePoints` (`self.Spline`)))
    (`self.SpawnAndSet` (`KismetMathLibrary.MakeTransform` (`KismetMathLibrary.MakeVector` (.x (.location (`SplineComponent.GetTransformAtSplinePoint` (`self.Spline`) _index "World" false))) (.y (.location (`SplineComponent.GetTransformAtSplinePoint` (`self.Spline`) _index "World" false))) (- (.z (.location (`SplineComponent.GetTransformAtSplinePoint` (`self.Spline`) _index "World" false))) (`self.HeightOffset`))) (`KismetMathLibrary.MakeRotator` (.roll (.rotation (`SplineComponent.GetTransformAtSplinePoint` (`self.Spline`) _index "World" false))) (.pitch (.rotation (`SplineComponent.GetTransformAtSplinePoint` (`self.Spline`) _index "World" false))) (+ (.yaw (.rotation (`SplineComponent.GetTransformAtSplinePoint` (`self.Spline`) _index "World" false))) (`self.Mesh_B_Rotation`)))) (`|GetArrayItem` _mesh_array (`KismetMathLibrary.RandomIntegerInRange` 0 (`KismetArrayLibrary.Array_Length` _mesh_array)))))
  (`self.K2_DestroyActor`))

(fn `Spawn_ElectricPoles`
  (params (PointIndex :type Integer))
  (bind _mesh_array (`self.Mesh_Array`))
  (bind _returnvalue (`|SpawnActorFromClass` "/Script/Engine.StaticMeshActor" (`KismetMathLibrary.MakeTransform` (`KismetMathLibrary.MakeVector` (.x (.location (`SplineComponent.GetTransformAtSplinePoint` (`self.Spline`) PointIndex "World" false))) (.y (.location (`SplineComponent.GetTransformAtSplinePoint` (`self.Spline`) PointIndex "World" false))) (- (.z (.location (`SplineComponent.GetTransformAtSplinePoint` (`self.Spline`) PointIndex "World" false))) (`self.HeightOffset`))) (`KismetMathLibrary.MakeRotator` (.roll (.rotation (`SplineComponent.GetTransformAtSplinePoint` (`self.Spline`) PointIndex "World" false))) (.pitch (.rotation (`SplineComponent.GetTransformAtSplinePoint` (`self.Spline`) PointIndex "World" false))) (+ (.yaw (.rotation (`SplineComponent.GetTransformAtSplinePoint` (`self.Spline`) PointIndex "World" false))) (`self.Mesh_B_Rotation`)))) "Undefined" "OverrideRootScale" null null))
  (`StaticMeshComponent.SetStaticMesh` (`StaticMeshActor.StaticMeshComponent` _returnvalue) (`|GetArrayItem` _mesh_array (`KismetMathLibrary.RandomIntegerInRange` 0 (`KismetArrayLibrary.Array_Length` _mesh_array)))))

(fn `SpawnAndSet`
  (params (InitTransform :type "Transform Structure") (mesh :type "StaticMesh Object Reference"))
  (bind _returnvalue (`|SpawnActorFromClass` "/Script/Engine.StaticMeshActor" InitTransform "AdjustIfPossibleButAlwaysSpawn" "OverrideRootScale" null null))
  (`StaticMeshComponent.SetStaticMesh` (`StaticMeshActor.StaticMeshComponent` _returnvalue) mesh))

(fn `UserConstructionScript`
  (locals (Index :type Integer) (Step :type Integer :default 3) (IndexToSet :type Integer))
  (bind _mesh_array (`self.Mesh_Array`))
  (for _index (range (`SplineComponent.GetNumberOfSplinePoints` (`self.Spline`)))
    (if (== (mod _index 2) 0)
      (bind (_returnvalue_location _returnvalue_rotation) (`KismetMathLibrary.BreakTransform` (`SplineComponent.GetTransformAtSplinePoint` (`self.Spline`) _index "Local" false)))
      (bind _returnvalue (`AddComponent|NODE_AddSpotLightComponent-0` :`RelativeTransform` (`KismetMathLibrary.MakeTransform` (`KismetMathLibrary.MakeVector` (.x _returnvalue_location) (+ (.y _returnvalue_location) (`self.light offste`)) (.z _returnvalue_location)) (`KismetMathLibrary.MakeRotator` (+ (.roll (`self.light rot`)) (.roll _returnvalue_rotation)) (+ (.pitch (`self.light rot`)) (.pitch _returnvalue_rotation)) (+ (.yaw (`self.light rot`)) (.yaw _returnvalue_rotation))))))
      (`LightComponent.SetLightColor` _returnvalue (`self.Light_Color`) true)
      (`LightComponent.SetIESBrightnessScale` _returnvalue (`self.Light_Intensity`))
      (`SpotLightComponent.SetOuterConeAngle` _returnvalue (`self.Light_OuterCone`))
      (`SpotLightComponent.SetInnerConeAngle` _returnvalue (`self.Light_InnerCone`)))
    (bind _returnvalue_2 (`AddComponent|NODE_AddSplineMeshComponent-8` :`RelativeTransform` (`KismetMathLibrary.MakeTransform` (`KismetMathLibrary.MakeVector` (.x _returnvalue_location) (.y _returnvalue_location) (- (.z _returnvalue_location) (`self.HeightOffset`))) (`KismetMathLibrary.MakeRotator` (.roll _returnvalue_rotation) (.pitch _returnvalue_rotation) (+ (.yaw _returnvalue_rotation) (`self.Mesh_B_Rotation`))) (0.1 1.0 1.0))))
    (`StaticMeshComponent.SetStaticMesh` _returnvalue_2 (`|GetArrayItem` _mesh_array (`KismetMathLibrary.RandomIntegerInRange` 0 (- (`KismetArrayLibrary.Array_Length` _mesh_array) 1))))))